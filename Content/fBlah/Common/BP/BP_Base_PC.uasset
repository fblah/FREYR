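; Base player controller that creates and shows the main menu and pause screen widgets, turning on the mouse cursor for each.
; BeginPlay opens the main menu when the current level matches the main menu level name, while the pause screen waits for its own event.
; Input actions drive the main menu: Up, Down and Left share an AddFocus call, Back calls GoBack and Right calls GoRight.
; Pause screen input branches are empty stubs.
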(event `ShowMainMenu`
  (`/Engine/EditorBlueprintResources/StandardMacros.IsValid` (`self.MainMenu`)
    (:`Is Valid`
      _)
    (:`Is Not Valid`
      (bind _returnvalue (`|CreateWidget` "/Game/UI/MainMenuUI.MainmenuUI_C" self))))
  (bind _output_get (set `self.MainMenu` _returnvalue))
  (`UserWidget.AddToViewport` _output_get 0)
  (set `self.bShowMouseCursor` true))

(event `self.ReceiveBeginPlay`
  (bind _returnvalue (`GameplayStatics.GetCurrentLevelName` true))
  (if (`KismetStringLibrary.EqualEqual_StrStr` _returnvalue (`self.MainMenuLevelName`))
    (`self.ShowMainMenu`)))

(event `ShowPauseScreen`
  (bind _returnvalue (`|CreateWidget` "/Game/UI/PauseUI.PauseUI_C" self))
  (`UserWidget.AddToViewport` _returnvalue 0)
  (set `self.PauseScreen` _returnvalue)
  (set `self.bShowMouseCursor` true))

(event `InputAction|Up` :paused true
  (params (Key :type "Key Structure"))
  (bind _pausescreen (`self.PauseScreen`))
  (bind _mainmenu (`self.MainMenu`))
  (:`Pressed`
    (`|ExecutionSequence` :!label _label
      (:`then_0`
        (`/Engine/EditorBlueprintResources/StandardMacros.IsValid` _mainmenu
          (:`Is Valid`
            (`/Game/UI/MainMenuUI.AddFocus` _mainmenu))))
      (:`then_1`
        (`/Engine/EditorBlueprintResources/StandardMacros.IsValid` _pausescreen
          (:`Is Valid`
            (if (`Widget.IsInViewport` _pausescreen)
              _)))))))

(event `InputAction|Down` :paused true
  (params (Key :type "Key Structure"))
  (:`Pressed`
    (goto _label)))

(event `InputAction|Left` :paused true
  (params (Key :type "Key Structure"))
  (:`Pressed`
    (goto _label)))

(event `InputAction|Back` :paused true
  (params (Key :type "Key Structure"))
  (bind _mainmenu (`self.MainMenu`))
  (:`Pressed`
    (`|ExecutionSequence`
      (:`then_0`
        (`/Engine/EditorBlueprintResources/StandardMacros.IsValid` _mainmenu
          (:`Is Valid`
            (`/Game/UI/MainMenuUI.GoBack` _mainmenu))))
      (:`then_1`
        (`/Engine/EditorBlueprintResources/StandardMacros.IsValid` (`self.PauseScreen`))))))

(event `InputAction|Right` :paused true
  (params (Key :type "Key Structure"))
  (bind _mainmenu (`self.MainMenu`))
  (:`Pressed`
    (`|ExecutionSequence`
      (:`then_0`
        (`/Engine/EditorBlueprintResources/StandardMacros.IsValid` _mainmenu
          (:`Is Valid`
            (`/Game/UI/MainMenuUI.GoRight` _mainmenu))))
      (:`then_1`
        (`/Engine/EditorBlueprintResources/StandardMacros.IsValid` (`self.PauseScreen`))))))

(fn `UserConstructionScript`)